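; Tank game mode Blueprint that puts up the UI for match start and match end.
; GameStart adds the HUD to the viewport, then calls a helper that creates the game start widget and hands it the StartDelay value.
; GameOver creates the game over widget, passes it whether the player won, and adds it to the viewport.
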(event EventGameStart
  (bind _returnvalue (UserInterface|CreateWidget "/Game/Blueprints/Widgets/WBP_HUD.WBP_HUD_C"))
  (UserInterface|Viewport|AddtoViewport _returnvalue 0)
  (CallFunction|CreateGameStartWidget))

(event EventGameOver
  (params (bPlayerWon :type Boolean))
  (bind _returnvalue (UserInterface|CreateWidget "/Game/Blueprints/Widgets/WBP_GameOver.WBP_GameOver_C"))
  (Default|SetPlayerWon _returnvalue bPlayerWon)
  (UserInterface|Viewport|AddtoViewport _returnvalue 0))

(fn ConstructionScript)

(fn CreateGameStartWidget
  (bind _returnvalue (UserInterface|CreateWidget "/Game/Blueprints/Widgets/WBP_GameStart.WBP_GameStart_C"))
  (Default|SetStartDelay _returnvalue (Variables|Default|GetStartDelay))
  (UserInterface|Viewport|AddtoViewport _returnvalue 0))