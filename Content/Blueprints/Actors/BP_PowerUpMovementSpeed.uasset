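; BP_PowerUpMovementSpeed is a power-up that temporarily doubles the movement speed of a PawnTank.
; ApplyBuf casts its target to PawnTank, stores the original MoveSpeed, applies the doubled value and starts a short timer by function name.
; When the timer fires, ResetMoveSpeed restores the stored speed on the saved target.
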(event EventApplyBuf
  (params (Target :type Actor%20Object%20Reference))
  (bind _aspawn_tank (Utilities|Casting|CastToPawnTank Target))
  (bind _output_get (Variables|Default|SetTarget _aspawn_tank))
  (bind _output_get_2 (Variables|Default|SetOriginalMoveSpeed (Variables|/Script/ToonTanks.PawnTank|GetMoveSpeed _output_get)))
  (Variables|/Script/ToonTanks.PawnTank|SetMoveSpeed _output_get (* 2.0 _output_get_2))
  (Utilities|Time|SetTimerbyFunctionName 0 "ResetMoveSpeed" 3.0))

(fn ConstructionScript)

(fn ResetMoveSpeed
  (Variables|/Script/ToonTanks.PawnTank|SetMoveSpeed (Variables|Default|GetTarget) (Variables|Default|GetOriginalMoveSpeed)))